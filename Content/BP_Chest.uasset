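; BP_Chest is an interactable chest that opens once the player has supplied two keys.
; On Interaction it checks the BP_Player's Keys array for each key in turn, revealing each held key and animating it sliding and rotating via a timeline.
; Each key sets a used flag, and the chain continues after the animation.
; When both flags are set, a final timeline pitches the cover open.
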(event `/Game/BPI_Interaction.Interaction`
  (bind _key1 (`self.Key1`))
  (bind _returnvalue (`SceneComponent.GetRelativeTransform` _key1))
  (if (`|GetArrayItem` (`/Game/BP_Player.Keys` (cast `/Game/BP_Player` (`GameplayStatics.GetPlayerCharacter` 0) :!pure true)))
    (`SceneComponent.SetVisibility` (`self.Key1`) true false)
    (set `self.Key1Used` true)
    (bind (_direction _movement _rotation) (`Timeline|Key1Movement`)
      (:`Update`
        (`SceneComponent.K2_SetRelativeLocationAndRotation` _key1 (`KismetMathLibrary.MakeVector` (`KismetMathLibrary.Lerp` 105.0 85.0 _movement) (.y (.location _returnvalue)) (.z (.location _returnvalue))) (`KismetMathLibrary.MakeRotator` (`KismetMathLibrary.Lerp` 0.0 90.0 _rotation) (.pitch (.rotation _returnvalue)) (.yaw (.rotation _returnvalue))) false false))
      (:`Finished`
        (`self.TestKey2`)))
    (else
      (`self.TestKey2`))))

(event `TestKey2`
  (bind _key2 (`self.Key2`))
  (bind _returnvalue (`SceneComponent.GetRelativeTransform` _key2))
  (if (`|GetArrayItem` (`/Game/BP_Player.Keys` (cast `/Game/BP_Player` (`GameplayStatics.GetPlayerCharacter` 0) :!pure true)) 1)
    (`SceneComponent.SetVisibility` (`self.Key2`) true false)
    (set `self.Key2Used` true)
    (bind (_direction _movement _rotation) (`Timeline|Timeline_0`)
      (:`Update`
        (`SceneComponent.K2_SetRelativeLocationAndRotation` _key2 (`KismetMathLibrary.MakeVector` (`KismetMathLibrary.Lerp` 105.0 85.0 _movement) (.y (.location _returnvalue)) (.z (.location _returnvalue))) (`KismetMathLibrary.MakeRotator` (`KismetMathLibrary.Lerp` 0.0 -90.0 _rotation) (.pitch (.rotation _returnvalue)) (.yaw (.rotation _returnvalue))) false false))
      (:`Finished`
        (`self.TestChest`)))))

(event `TestChest`
  (if (and (`self.Key1Used`) (`self.Key2Used`))
    (bind (_direction _newtrack_0) (`Timeline|Timeline`)
      (:`Update`
        (`SceneComponent.K2_SetRelativeRotation` (`self.Chest_cover6_StaticMeshComponent0`) (`KismetMathLibrary.MakeRotator` 0.0 (* _newtrack_0 60.0)) false false)))))

(fn `UserConstructionScript`)