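; Player character Blueprint that lets the player pick an overlapping item and inspect its mesh.
; E queries overlapping actors through BPI_interface, shows the returned static mesh on InspectItemModel and zeroes walk speed.
; While viewing, holding H pitches the model steadily on Tick, and J hides it and restores walk speed.
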(event `self.ReceiveTick`
  (params (DeltaSeconds :type "Float (single-precision)"))
  (if (`self.RotatingModel`)
    (`SceneComponent.K2_AddLocalRotation` (`self.Inspect Item Model`) (`KismetMathLibrary.MakeRotator` 0.0 (* DeltaSeconds 10.0)) false false)))

(event `Key|H`
  (params (Key :type "Key Structure"))
  (:`Pressed`
    (if (`self.IsViewingItem`)
      (set `self.RotatingModel` true)))
  (:`Released`
    (set `self.RotatingModel` false)))

(event `Key|J`
  (params (Key :type "Key Structure"))
  (:`Pressed`
    (if (`self.IsViewingItem`)
      (`SceneComponent.SetVisibility` (`self.Inspect Item Model`) false false)
      (set `CharacterMovementComponent.MaxWalkSpeed` 500.0 (`self.CharacterMovement`))
      (set `self.IsViewingItem` false))))

(event `Key|E`
  (params (Key :type "Key Structure"))
  (bind _inspect_item_model (`self.Inspect Item Model`))
  (:`Pressed`
    (for _array_element (`self.GetOverlappingActors` null)
      (if (`KismetSystemLibrary.DoesClassImplementInterface` (`GameplayStatics.GetObjectClass` _array_element) "/Game/exercice/BPI_interface.BPI_interface_C")
        (bind _itemmodel (message `/Game/exercice/BPI_interface.InteractItem` _array_element))
        (`StaticMeshComponent.SetStaticMesh` _inspect_item_model _itemmodel)
        (`SceneComponent.SetVisibility` _inspect_item_model true false)
        (set `self.IsViewingItem` true)
        (set `CharacterMovementComponent.MaxWalkSpeed` 0.0 (`self.CharacterMovement`))))))

(fn `UserConstructionScript`)