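; BP_inspection is an interactable item actor that can be grabbed, handing over its model and then removing itself from the level.
; The construction script applies the ItemModel variable to its static mesh component.
; InteractItem prints a grab message, triggers DestroyItem, which destroys the actor after a short delay, and returns ItemModel to the caller.
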(event `DestroyItem`
  (`KismetSystemLibrary.Delay` 0.2)
  (`self.K2_DestroyActor`))

(fn `InteractItem`
  (returns (ItemModel :type "StaticMesh Object Reference"))
  (`KismetSystemLibrary.PrintString` "Item Grabbed")
  (`self.DestroyItem`)
  (return (`self.ItemModel`)))

(fn `UserConstructionScript`
  (`StaticMeshComponent.SetStaticMesh` (`self.StaticMesh`) (`self.ItemModel`)))