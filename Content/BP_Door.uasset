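; Double-leaf door actor that swings two meshes open and closed in opposite directions, 80 degrees each.
; The openDoor event toggles IsClosed, playing or reversing the RotationDoor timeline that drives both meshes' yaw.
; The construction script poses the meshes and timeline from IsClosed, though its yaw values are swapped between the two meshes compared with the timeline.
; Older FlipFlop and instant-rotation logic remains unconnected.
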(event `self.ReceiveBeginPlay`
  ;[1 1 1] Comment
)

(event `openDoor`
  ;[1 1 1] Comment
  (if (`self.IsClosed`)
    (set `self.IsClosed` false)
    (bind (_direction _rotation_value) (`Timeline|rotationDoor` :!label _label)
      (:`Update`
        (`SceneComponent.K2_SetRelativeRotation` (`self.Door_3_StaticMeshComponent1`) (`KismetMathLibrary.MakeRotator` 0.0 0.0 (* _rotation_value -80.0)) false false)
        (`SceneComponent.K2_SetRelativeRotation` (`self.Door_3_StaticMeshComponent0`) (`KismetMathLibrary.MakeRotator` 0.0 0.0 (`KismetMathLibrary.Lerp` 180.0 260.0 _rotation_value)) false false)))
    (else
      (set `self.IsClosed` true)
      (goto _label :!via `Reverse`))))

(fn `UserConstructionScript`
  (`SceneComponent.K2_SetRelativeRotation` (`self.Door_3_StaticMeshComponent1`) (`KismetMathLibrary.MakeRotator` 0.0 0.0 (select `bool` (`self.IsClosed`) :`false` 260.0 :`true` 180.0)) false false)
  (`SceneComponent.K2_SetRelativeRotation` (`self.Door_3_StaticMeshComponent0`) (`KismetMathLibrary.MakeRotator` 0.0 0.0 (select `bool` (`self.IsClosed`) :`false` -80.0)) false false)
  (`TimelineComponent.SetNewTime` (`self.rotationDoor`) (select `bool` (`self.IsClosed`) :`false` 1.0)))